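; Enemy character for the Motion Combat System, driven by a State Tree AI controller on perception team 2.
; It is always targetable and answers combat damage with a severity-based hit reaction, without applying damage itself.
; Health changes update a widget healthbar, whose camera-facing update is never called.
; Global combat event bus handlers only print debug text; death stops the State Tree, and EndPlay also clears bindings.
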(event Custom|On%20Attack%20Started
  (params (Attacker :type Actor%20Object%20Reference) (Target :type Actor%20Object%20Reference))
  (Development|PrintText (Utilities|Text|FormatText "Attack Started:  
- Attacker | {A} 
- Target | {T}" (Utilities|GetDisplayName Attacker) (Utilities|GetDisplayName Target)) true true "(R=0.000000,G=0.000000,B=0.000000,A=1.000000)"))

(event Custom|On%20Parry%20Success
  (params (Defender :type Actor%20Object%20Reference) (Attacker :type Actor%20Object%20Reference))
  (Development|PrintText (Utilities|Text|FormatText "On Parry Success:  
- Defender | {A} 
- Attacker | {T}" (Utilities|GetDisplayName Defender) (Utilities|GetDisplayName Attacker)) true true "(R=0.000000,G=0.000000,B=0.000000,A=1.000000)"))

(event Custom|On%20Hit%20Landed
  (params (Attacker :type Actor%20Object%20Reference) (Defender :type Actor%20Object%20Reference) (AttackData :type MCS%20Attack%20Entry%20Structure%20%28by%20ref%29))
  (Development|PrintText (Utilities|Text|FormatText "On Hit Landed:  
- Defender | {A} 
- Attacker | {T}" (Utilities|GetDisplayName Attacker) (Utilities|GetDisplayName Defender)) true true "(R=0.000000,G=0.000000,B=0.000000,A=1.000000)"))

(event Custom|On%20Parry%20Window%20Open
  (params (Attacker :type Actor%20Object%20Reference) (Duration :type Float%20%28single-precision%29))
  (Development|PrintText (Utilities|Text|FormatText "On Parry Window Open:  
- Defender | {A} 
- Duration | {D}" (Utilities|GetDisplayName Attacker) Duration) true true "(R=0.000000,G=0.000000,B=0.000000,A=1.000000)"))

(event EventBeginPlay
  ;[1 1 1] Bind Event Bus Events
  (CallFunction|AssignGlobalEventBusEvents)
  ;[1 1 1] Get AI Controller
  (bind _asmotion_combat_enemy_ai_controller (Utilities|Casting|CastToMC_EnemyAIController (AI|GetAIController 0)))
  (Variables|Default|SetAIC _asmotion_combat_enemy_ai_controller)
  ;[1 1 1] Set team ID so AI perception knows who is friendly or not
  (Class|MCCharacterBase|SetTeamID 2))

(event EventEndPlay
  (params (EndPlayReason :type EEndPlayReason%20Enum :default "Destroyed"))
  ;[1 1 1] Clean up bindings
  (CallFunction|HandleEndPlay))

(event EventOnCharacterDamageTaken
  (params (DamageAmount :type Float%20%28single-precision%29) (NewHealth :type Float%20%28single-precision%29) (InstigatorActor :type Actor%20Object%20Reference)))

(event EventOnCharacterHealthChanged
  (params (NewHealth :type Float%20%28single-precision%29) (MaxHealth :type Float%20%28single-precision%29))
  ;[1 1 1] Update health bar
  (CallFunction|UpdateHealthbar NewHealth MaxHealth))

(event EventOnCharacterDeath
  (params (DeadActor :type Actor%20Object%20Reference))
  ;[1 1 1] Stop state tree logic on death
  (bind _aic (Variables|Default|GetAIC)
    (:then
      (Class|MCStateTreeAIComponent|StopStateTree (Variables|/Script/MotionCombat.MC_EnemyAIController|GetStateTreeAIComponent _aic)))
    (:else)))

(event EventTick
  (params (DeltaSeconds :type Float%20%28single-precision%29)))

(fn ConstructionScript)

(fn AssignGlobalEventBusEvents
  (bind _returnvalue (Class|MCSCombatEventBus|GetCombatEventBus))
  (Utilities|FlowControl|Sequence
    (:then_0
      (EventDispatchers|BindEventtoOnAttackStarted _returnvalue (EventDispatchers|CreateEvent :!event Custom|On%20Attack%20Started)))
    (:then_1
      (EventDispatchers|BindEventtoOnParrySuccess _returnvalue (EventDispatchers|CreateEvent :!event Custom|On%20Parry%20Success)))
    (:then_2
      (EventDispatchers|BindEventtoOnHitLanded _returnvalue (EventDispatchers|CreateEvent :!event Custom|On%20Hit%20Landed)))
    (:then_3
      (EventDispatchers|BindEventtoOnParryWindowOpened _returnvalue (EventDispatchers|CreateEvent :!event Custom|On%20Parry%20Window%20Open)))))

(fn GetMCSHitboxComponent
  (bind _motion_combat_system_hitbox_component (Variables|Default|GetMotion%20Combat%20System%20Hitbox%20Component)
    (:then
      (return _motion_combat_system_hitbox_component))
    (:else
      (return 0))))

(fn GetMCSCoreComponent
  (bind _motion_combat_system_core_component (Variables|Default|GetMotion%20Combat%20System%20Core%20Component)
    (:then
      (return _motion_combat_system_core_component))
    (:else
      (return 0))))

(fn GetCharacterAnimInstance
  (bind _mesh (Variables|Character|GetMesh)
    (:then
      (return (Components|SkeletalMesh|GetAnimInstance _mesh)))
    (:else
      (return 0))))

(fn GetHitReactionComponent
  (bind _motion_combat_system_hit_reaction_component (Variables|Default|GetMotion%20Combat%20System%20Hit%20Reaction%20Component)
    (:then
      (return _motion_combat_system_hit_reaction_component))
    (:else
      (return 0))))

(fn GetMCSDefenseComponent
  (bind _motion_combat_system_combat_defense_component (Variables|Default|GetMotion%20Combat%20System%20Combat%20Defense%20Component)
    (:then
      (return _motion_combat_system_combat_defense_component))
    (:else
      (return 0))))

(fn UnAssignGlobalEventBusEvents
  (bind _returnvalue (Class|MCSCombatEventBus|GetCombatEventBus))
  (Utilities|FlowControl|Sequence
    (:then_0
      (EventDispatchers|UnbindEventfromOnAttackStarted _returnvalue (EventDispatchers|CreateEvent :!event Custom|On%20Attack%20Started)))
    (:then_1
      (EventDispatchers|UnbindEventfromOnParrySuccess _returnvalue (EventDispatchers|CreateEvent :!event Custom|On%20Parry%20Success)))
    (:then_2
      (EventDispatchers|UnbindEventfromOnHitLanded _returnvalue (EventDispatchers|CreateEvent :!event Custom|On%20Hit%20Landed)))
    (:then_3
      (EventDispatchers|UnbindEventfromOnParryWindowOpened _returnvalue (EventDispatchers|CreateEvent :!event Custom|On%20Parry%20Window%20Open)))))

(fn HandleEndPlay
  (Utilities|FlowControl|Sequence
    (:then_0
      (CallFunction|UnAssignGlobalEventBusEvents))
    (:then_1
      (bind _aic (Variables|Default|GetAIC)
        (:then
          (Class|MCStateTreeAIComponent|StopStateTree (Variables|/Script/MotionCombat.MC_EnemyAIController|GetStateTreeAIComponent _aic)))
        (:else)))
    (:then_2
      (bind _aic_2 (Variables|Default|GetAIC)
        (:then
          (EventDispatchers|UnbindallEventsfromOnDamageStimulusEvent _aic_2)
          (EventDispatchers|UnbindallEventsfromOnHearingStimulusEvent _aic_2)
          (EventDispatchers|UnbindallEventsfromOnHearingStimulusForgottenEvent _aic_2)
          (EventDispatchers|UnbindallEventsfromOnSightStimulusEvent _aic_2)
          (EventDispatchers|UnbindallEventsfromOnSightStimulusForgottenEvent _aic_2))
        (:else)))))

(fn OrientHealthbartoCamera
  (bind _healthbar (Variables|Default|GetHealthbar))
  (Transformation|SetWorldRotation _healthbar (Math|Rotator|FindLookatRotation (Transformation|GetWorldLocation _healthbar) (Camera|GetCameraLocation (Game|GetPlayerCameraManager 0))) false false))

(fn UpdateHealthbar
  (params (Health :type Float%20%28double-precision%29) (MaxHealth :type Float%20%28double-precision%29))
  (bind _healthbar (Variables|Default|GetHealthbar)
    (:then
      (bind _aswbp_healthbar (Utilities|Casting|CastToWBP_Healthbar (UserInterface|GetWidget _healthbar)))
      (Default|UpdateHealthbar _aswbp_healthbar (Math|Float|Clamp(Float) (/ Health MaxHealth))))
    (:else)))

(fn CanbeTargeted
  (return true))

(fn TakeCombatDamage
  (params (Damage :type Float%20%28single-precision%29) (Hit :type Hit%20Result%20Structure%20%28by%20ref%29) (AttackEntry :type MCS%20Attack%20Entry%20Structure%20%28by%20ref%29))
  (Utilities|FlowControl|Sequence
    (:then_0)
    (:then_1
      ;[1 1 1] Handle hit reaction
      (Class|MCSCombatHitReactionComponent|PerformHitReaction (Variables|Default|GetMotion%20Combat%20System%20Hit%20Reaction%20Component) Hit self (Utilities|Struct|BreakMCS_AttackEntry AttackEntry)))
    (:then_2
      (return true))))