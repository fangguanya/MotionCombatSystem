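; Idle state node for enemy AI that holds until the controller's AI state changes, with no idle behavior of its own.
; On enter it caches the enemy controller, pawn and combat character base, and on exit it clears them.
; Each tick prints a debug message and finishes the node successfully once the controller's current state is no longer Idle.
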(event EventOnEnterNode
  (params (OwnerController :type AI%20Controller%20Object%20Reference) (ControlledPawn :type Pawn%20Object%20Reference))
  (bind _asmotion_combat_enemy_ai_controller (Utilities|Casting|CastToMC_EnemyAIController OwnerController))
  (Variables|Default|SetEnemy%20AI%20Controller _asmotion_combat_enemy_ai_controller)
  (bind _output_get (Variables|Default|SetEnemy%20Pawn ControlledPawn))
  (bind _asmotion_combat_character_base (Utilities|Casting|CastToMC_CharacterBase _output_get))
  (Variables|Default|SetCombat%20Character%20Base _asmotion_combat_character_base))

(event EventOnTickNode
  (params (OwnerController :type AI%20Controller%20Object%20Reference) (ControlledPawn :type Pawn%20Object%20Reference) (DeltaTime :type Float%20%28single-precision%29))
  (Development|PrintString 0 "Ticking Idle Mode" true false "(R=0.000000,G=0.000000,B=0.000000,A=1.000000)" 2.0 "Tick")
  (if (not (Utilities|Enum|Equal(Enum) (Variables|/Script/MotionCombat.MC_EnemyAIController|GetCurrentAIState (Variables|Default|GetEnemy%20AI%20Controller)) "Idle"))
    (Class|MCAINodeBase|FinishNode true)))

(event EventOnExitNode
  (params (OwnerController :type AI%20Controller%20Object%20Reference) (ControlledPawn :type Pawn%20Object%20Reference))
  (Variables|Default|SetEnemy%20AI%20Controller 0)
  (Variables|Default|SetEnemy%20Pawn 0)
  (Variables|Default|SetCombat%20Character%20Base 0))