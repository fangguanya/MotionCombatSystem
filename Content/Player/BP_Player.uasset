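; Player character Blueprint for the Motion Combat System (MCS), starting with the unarmed attack set and caching its player controller on possession.
; Hitbox hits on characters implementing the combat interface send damage with the attack entry and print bone debug text.
; Incoming damage only triggers a hit reaction at the attack's severity, with no health change.
; Interface getters expose the core, hitbox, defense and hit reaction components, and the player cannot be targeted.
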(event OnTargetingUpdated(MotionCombatSystemCoreComponent)
  (params (NewTargetList :type Array%20of%20MCS%20Target%20Info%20Structures) (NumTargets :type Integer)))

(event OnHitboxHit(MotionCombatSystemHitboxComponent)
  (params (HitActor :type Actor%20Object%20Reference) (HitResult :type Hit%20Result%20Structure%20%28by%20ref%29) (AttackEntry :type MCS%20Attack%20Entry%20Structure))
  (bind (_bblockinghit _binitialoverlap _time _distance _location _impactpoint _normal _impactnormal _physmat _hitactor _hitcomponent _hitbonename _bonename _hititem) (Collision|BreakHitResult HitResult))
  ;[1 1 1] Send damage to hit actor
  (Class|KismetSystemLibrary|IsObjectOfSoftClass HitActor "/Script/Engine.Character"
    (:True
      (if (Utilities|DoesObjectImplementInterface HitActor "/Script/MotionCombatSystem.MCS_CombatCharacterInterface")
        (Class|MCSCombatCharacterInterface|TakeCombatDamage(Message) HitActor (.Damage (Utilities|Struct|BreakMCS_AttackEntry AttackEntry)) HitResult AttackEntry)
        (Development|PrintText (Utilities|Text|FormatText "Hit Bone Name: {HitBone} 
Bone Name: {BoneName} 
Hit Item: {HitItem}" _hitbonename _bonename _hititem) true true "(R=0.000000,G=0.000000,B=0.000000,A=1.000000)")))))

(event EventBeginPlay
  ;[1 1 1] Start with unarmed attack set
  (CallFunction|SetActiveAttackSetbyTag "(TagName=\"MCS.Attacks.Unarmed\")"))

(event EventPossessed
  (params (NewController :type Controller%20Object%20Reference))
  (if (Class|Controller|IsPlayerController NewController)
    (bind _asbp_player_controller (Utilities|Casting|CastToBP_PlayerController NewController))
    (Variables|Default|SetMyPlayerController _asbp_player_controller)))

(fn ConstructionScript)

(fn GetMCSHitboxComponent
  (bind _motion_combat_system_hitbox_component (Variables|Default|GetMotion%20Combat%20System%20Hitbox%20Component)
    (:then
      (return _motion_combat_system_hitbox_component))
    (:else
      (return 0))))

(fn GetMCSCoreComponent
  (bind _motion_combat_system_core_component (Variables|Default|GetMotion%20Combat%20System%20Core%20Component)
    (:then
      (return _motion_combat_system_core_component))
    (:else
      (return 0))))

(fn SetActiveAttackSetbyTag
  (params (Tag :type Gameplay%20Tag%20Structure))
  (bind _returnvalue (Class|MCSCombatCoreComponent|SetActiveAttackSet (Variables|Default|GetMotion%20Combat%20System%20Core%20Component) Tag))
  (return _returnvalue))

(fn GetCharacterAnimInstance
  (bind _mesh (Variables|Character|GetMesh)
    (:then
      (return (Components|SkeletalMesh|GetAnimInstance _mesh)))
    (:else
      (return 0))))

(fn GetHitReactionComponent
  (bind _motion_combat_system_hit_reaction_component (Variables|Default|GetMotion%20Combat%20System%20Hit%20Reaction%20Component)
    (:then
      (return _motion_combat_system_hit_reaction_component))
    (:else
      (return 0))))

(fn GetMCSDefensseComponent
  (bind _motion_combat_system_defense_component (Variables|Default|GetMotion%20Combat%20System%20Defense%20Component)
    (:then
      (return _motion_combat_system_defense_component))
    (:else
      (return 0))))

(fn CanbeTargeted
  (return false))

(fn TakeCombatDamage
  (params (Damage :type Float%20%28single-precision%29) (Hit :type Hit%20Result%20Structure%20%28by%20ref%29) (AttackEntry :type MCS%20Attack%20Entry%20Structure%20%28by%20ref%29))
  (Utilities|FlowControl|Sequence
    (:then_0)
    (:then_1
      ;[1 1 1] Handle hit reaction
      (Class|MCSCombatHitReactionComponent|PerformHitReaction (Variables|Default|GetMotion%20Combat%20System%20Hit%20Reaction%20Component) Hit self (Utilities|Struct|BreakMCS_AttackEntry AttackEntry)))
    (:then_2
      (return true))))